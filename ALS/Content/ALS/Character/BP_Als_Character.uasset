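; ALS character Blueprint that shows held props such as weapons, tools and carried objects to match the current overlay mode.
; Overlay changes refresh the socket-attached static and skeletal mesh components; ragdolling and non-low mantles clear them until finished.
; While in Bow mode, Tick feeds an animation curve into the bow AnimBP's Draw value.
; Selector functions choose mantling settings and get-up and roll montages suited to each overlay.
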(event EventTick
  (params (DeltaSeconds :type Float%20%28single-precision%29))
  (Overlay|TickOverlayObject))

(event EventOnOverlayModeChanged
  (params (PreviousMode :type EAlsOverlayMode%20Enum :default "Default"))
  (Overlay|RefreshOverlayObject))

(event EventOnMantlingEnded
  (Overlay|RefreshOverlayObject))

(event EventOnRagdollingEnded
  (Overlay|RefreshOverlayObject))

(event EventOnMantlingStarted
  (params (TargetPrimitive :type Primitive%20Component%20Object%20Reference) (TargetLocation :type Vector%20%28by%20ref%29 :default "0, 0, 0") (TargetRotation :type Rotator%20%28by%20ref%29 :default "0, 0, 0") (MantlingHeight :type Float%20%28single-precision%29) (MantlingType :type EAlsMantlingType%20Enum :default "High"))
  (if (Utilities|Enum|NotEqual(Enum) MantlingType "Low")
    (Overlay|ClearOverlayObject)))

(event EventBeginPlay
  (Overlay|RefreshOverlayObject))

(event EventOnRagdollingStarted
  (Overlay|ClearOverlayObject))

(fn ConstructionScript)

(fn RefreshOverlayObject
  (switch Utilities|FlowControl|Switch|SwitchonEAlsOverlayMode (Variables|Default|GetOverlayMode)
    (:Default
      (Overlay|ClearOverlayObject :!label _label))
    (:Masculine
      (goto _label))
    (:Feminine
      (goto _label))
    (:Injured
      (goto _label))
    (:HandsTied
      (goto _label))
    (:M4
      (Overlay|AttachOverlayObject 0 "/ALS/ALS/OverlayObjects/M4/SK_M4.SK_M4" 0 "M4" false false))
    (:PistolOneHanded
      (Overlay|AttachOverlayObject 0 "/ALS/ALS/OverlayObjects/M9/SK_M9.SK_M9" 0 "M9" false false))
    (:PistolTwoHanded
      (Overlay|AttachOverlayObject 0 "/ALS/ALS/OverlayObjects/M9/SK_M9.SK_M9" 0 "M9" false false))
    (:Bow
      (Overlay|AttachOverlayObject 0 "/ALS/ALS/OverlayObjects/Bow/SK_Bow.SK_Bow" "/ALS/ALS/OverlayObjects/Bow/ABP_Bow.ABP_Bow_C" "Bow" false true))
    (:Torch
      (Overlay|AttachOverlayObject "/ALS/ALS/OverlayObjects/Torch/S_Torch.S_Torch" 0 0 "Torch" false true))
    (:Binoculars
      (Overlay|AttachOverlayObject "/ALS/ALS/OverlayObjects/Binoculars/S_Binoculars.S_Binoculars" 0 0 "Binoculars" false false))
    (:Box
      (Overlay|AttachOverlayObject "/ALS/ALS/OverlayObjects/Box/S_Box.S_Box" 0 0 "Box" false false))
    (:Barrel
      (Overlay|AttachOverlayObject "/ALS/ALS/OverlayObjects/Barrel/S_Barrel.S_Barrel" 0 0 "Barrel" false true))))

(fn AttachOverlayObject
  (params (NewStaticMesh :type Static%20Mesh%20Object%20Reference) (NewSkeletalMesh :type Skeletal%20Mesh%20Object%20Reference) (NewAnimationClass :type Anim%20Instance%20Class%20Reference) (SocketName :type Name) (bAttachToGunBone :type Boolean) (bUseLeftGunBone :type Boolean))
  (LocalVariables|SetResultSocketName (select bAttachToGunBone (select bUseLeftGunBone (Class|AlsConstants|GunLeftVirtualBone) (Class|AlsConstants|GunRightVirtualBone)) SocketName))
  (Utilities|FlowControl|Sequence
    (:then_0
      (Components|StaticMesh|SetStaticMesh (Variables|Default|GetOverlayStaticMesh) NewStaticMesh)
      (Transformation|AttachComponentToComponent (Variables|Default|GetOverlayStaticMesh) (Variables|Character|GetMesh) SocketName "SnapToTarget" "SnapToTarget" "SnapToTarget" true))
    (:then_1
      (Class|SkinnedMeshComponent|SetSkeletalMesh (Variables|Default|GetOverlaySkeletalMesh) NewSkeletalMesh true)
      (Class|SkeletalMeshComponent|SetAnimClass (Variables|Default|GetOverlaySkeletalMesh) NewAnimationClass)
      (Transformation|AttachComponentToComponent (Variables|Default|GetOverlaySkeletalMesh) (Variables|Character|GetMesh) SocketName "SnapToTarget" "SnapToTarget" "SnapToTarget" true))))

(fn ClearOverlayObject
  (Components|StaticMesh|SetStaticMesh (Variables|Default|GetOverlayStaticMesh) 0)
  (Class|SkinnedMeshComponent|SetSkeletalMesh (Variables|Default|GetOverlaySkeletalMesh) 0 true)
  (Class|SkeletalMeshComponent|SetAnimClass (Variables|Default|GetOverlaySkeletalMesh)))

(fn TickOverlayObject
  (if (Utilities|Enum|Equal(Enum) (Variables|Default|GetOverlayMode) "Bow")
    (bind _asabp_bow (Utilities|Casting|CastToABP_Bow (Components|SkeletalMesh|GetAnimInstance (Variables|Default|GetOverlaySkeletalMesh))))
    (Variables|/ALS/ALS/OverlayObjects/Bow/ABP_Bow.ABP_Bow_C|SetDraw _asabp_bow (Class|AlsUtility|GetAnimationCurveValue 0 (Class|AlsConstants|AimManualCurve)))))

(fn SelectMantlingSettings
  (params (MantlingType :type EAlsMantlingType%20Enum :default "High"))
  (bind _mantlinghigh (Variables|Settings|AlsCharacter|Mantling|GetMantlingHigh))
  (bind _mantlinglow (Variables|Settings|AlsCharacter|Mantling|GetMantlingLow))
  (bind _mantlinglowleft (Variables|Settings|AlsCharacter|Mantling|GetMantlingLowLeft))
  (bind _mantlinglowright (Variables|Settings|AlsCharacter|Mantling|GetMantlingLowRight))
  (return (Utilities|Select :Index MantlingType :High _mantlinghigh :Low (Utilities|Select :Index (Variables|Default|GetOverlayMode) :Default _mantlinglow :Masculine _mantlinglow :Feminine _mantlinglow :Injured _mantlinglowleft :HandsTied (Variables|Settings|AlsCharacter|Mantling|GetMantlingLowBothHands) :M4 _mantlinglowright :PistolOneHanded _mantlinglowright :PistolTwoHanded _mantlinglowright :Bow _mantlinglowleft :Torch _mantlinglowleft :Binoculars _mantlinglowright :Box (Variables|Settings|AlsCharacter|Mantling|GetMantlingLowBox) :Barrel _mantlinglowleft) :InAir _mantlinghigh)))

(fn SelectGetUpMontage
  (params (bRagdollFacedUpward :type Boolean))
  (bind _getupback (Variables|Settings|AlsCharacter|GetUp|GetGetUpBack))
  (bind _getupbackrightarm (Variables|Settings|AlsCharacter|GetUp|GetGetUpBackRightArm))
  (bind _getupbackleftarm (Variables|Settings|AlsCharacter|GetUp|GetGetUpBackLeftArm))
  (bind _getupfront (Variables|Settings|AlsCharacter|GetUp|GetGetUpFront))
  (bind _getupfrontrigharm (Variables|Settings|AlsCharacter|GetUp|GetGetUpFrontRighArm))
  (bind _getupfrontleftarm (Variables|Settings|AlsCharacter|GetUp|GetGetUpFrontLeftArm))
  (return (select bRagdollFacedUpward (Utilities|Select :Index (Variables|Default|GetOverlayMode) :Default _getupback :Masculine _getupback :Feminine _getupback :Injured (Variables|Settings|AlsCharacter|GetUp|GetGetUpBackLeftArm) :HandsTied (Variables|Settings|AlsCharacter|GetUp|GetGetUpBackBothArms) :M4 _getupbackrightarm :PistolOneHanded _getupbackrightarm :PistolTwoHanded _getupbackrightarm :Bow _getupbackleftarm :Torch _getupbackleftarm :Binoculars (Variables|Settings|AlsCharacter|GetUp|GetGetUpBackRightArm) :Box (Variables|Settings|AlsCharacter|GetUp|GetGetUpBackBothArms) :Barrel (Variables|Settings|AlsCharacter|GetUp|GetGetUpBackLeftArm)) (Utilities|Select :Index (Variables|Default|GetOverlayMode) :Default _getupfront :Masculine _getupfront :Feminine _getupfront :Injured (Variables|Settings|AlsCharacter|GetUp|GetGetUpFrontLeftArm) :HandsTied (Variables|Settings|AlsCharacter|GetUp|GetGetUpFrontBothArms) :M4 _getupfrontrigharm :PistolOneHanded _getupfrontrigharm :PistolTwoHanded _getupfrontrigharm :Bow _getupfrontleftarm :Torch _getupfrontleftarm :Binoculars (Variables|Settings|AlsCharacter|GetUp|GetGetUpFrontRighArm) :Box (Variables|Settings|AlsCharacter|GetUp|GetGetUpFrontBothArms) :Barrel (Variables|Settings|AlsCharacter|GetUp|GetGetUpFrontLeftArm)))))

(fn SelectRollMontage
  (bind _roll (Variables|Settings|AlsCharacter|Roll|GetRoll))
  (bind _rollbotharms (Variables|Settings|AlsCharacter|Roll|GetRollBothArms))
  (bind _rollrightarm (Variables|Settings|AlsCharacter|Roll|GetRollRightArm))
  (bind _rollleftarm (Variables|Settings|AlsCharacter|Roll|GetRollLeftArm))
  (bind _rollbotharms_2 (Variables|Settings|AlsCharacter|Roll|GetRollBothArms))
  (return (Utilities|Select :Index (Variables|Default|GetOverlayMode) :Default _roll :Masculine _roll :Feminine _roll :Injured (Variables|Settings|AlsCharacter|Roll|GetRollLeftArm) :HandsTied _rollbotharms :M4 _rollbotharms :PistolOneHanded _rollrightarm :PistolTwoHanded _rollrightarm :Bow _rollleftarm :Torch _rollleftarm :Binoculars _rollbotharms_2 :Box _rollbotharms_2 :Barrel (Variables|Settings|AlsCharacter|Roll|GetRollLeftArm))))