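; Player controller for an ALS sample that creates the HUD and an overlay mode menu for the local player.
; Holding Q shows the menu and slows time, mouse wheel or D-pad cycles overlay modes, and release approves the choice.
; Tab flips a UI visibility flag and Z toggles persistent slow motion, which overrides the menu's slowdown.
; A wrapper function limits global time dilation changes to standalone games.
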(event EventBeginPlay
  (if (Pawn|IsLocalController)
    (Input|SetInputModeGameOnly self)
    (bind _returnvalue (UserInterface|CreateWidget "/ALS/ALSExtras/UI/WBP_Hud.WBP_Hud_C" self))
    (UserInterface|Viewport|AddtoViewport _returnvalue 0)
    (bind _returnvalue_2 (UserInterface|CreateWidget "/ALS/ALSExtras/UI/WBP_OverlayModeMenu.WBP_OverlayModeMenu_C" self))
    (Variables|State|SetOverlayModeMenuWidget _returnvalue_2)))

(event Input|KeyboardEvents|Z
  (params (Key :type Key%20Structure))
  (:Pressed
    (Variables|State|SetbSlomoActive (not (Variables|State|GetbSlomoActive)))
    (CallFunction|SetGlobalTimeDilation (Math|Float|SelectFloat 0.15 1.0 (Variables|State|GetbSlomoActive)))))

(event Input|KeyboardEvents|Tab
  (params (Key :type Key%20Structure))
  (:Pressed
    (Variables|State|SetbUIVisible (not (Variables|State|GetbUIVisible)))))

(event Input|KeyboardEvents|Q
  (params (Key :type Key%20Structure))
  (:Pressed
    (if (Variables|State|GetbSlomoActive)
      _
      (else
        (CallFunction|SetGlobalTimeDilation 0.35)))
    (UserInterface|Viewport|AddtoViewport (Variables|State|GetOverlayModeMenuWidget) 0))
  (:Released
    (if (Variables|State|GetbSlomoActive)
      _
      (else
        (CallFunction|SetGlobalTimeDilation 1.0)))
    (Default|ApproveOverlayMode (Variables|State|GetOverlayModeMenuWidget))
    (Widget|RemovefromParent (Variables|State|GetOverlayModeMenuWidget))))

(event Input|MouseEvents|MouseWheelUp
  (params (Key :type Key%20Structure))
  (:Pressed
    (if (UserInterface|Viewport|IsinViewport (Variables|State|GetOverlayModeMenuWidget))
      (Default|CycleOverlayMode (Variables|State|GetOverlayModeMenuWidget) true))))

(event Input|GamepadEvents|GamepadDPadUp
  (params (Key :type Key%20Structure))
  (:Pressed
    (if (UserInterface|Viewport|IsinViewport (Variables|State|GetOverlayModeMenuWidget))
      (Default|CycleOverlayMode (Variables|State|GetOverlayModeMenuWidget) true))))

(event Input|MouseEvents|MouseWheelDown
  (params (Key :type Key%20Structure))
  (:Pressed
    (if (UserInterface|Viewport|IsinViewport (Variables|State|GetOverlayModeMenuWidget))
      (Default|CycleOverlayMode (Variables|State|GetOverlayModeMenuWidget) false))))

(event Input|GamepadEvents|GamepadDPadDown
  (params (Key :type Key%20Structure))
  (:Pressed
    (if (UserInterface|Viewport|IsinViewport (Variables|State|GetOverlayModeMenuWidget))
      (Default|CycleOverlayMode (Variables|State|GetOverlayModeMenuWidget) false))))

(fn ConstructionScript)

(fn SetGlobalTimeDilation
  (params (Time%20Dilation :type Float%20%28double-precision%29))
  (if (Class|KismetSystemLibrary|IsStandalone)
    (Utilities|Time|SetGlobalTimeDilation Time%20Dilation)))