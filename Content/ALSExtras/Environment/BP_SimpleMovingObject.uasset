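; BP_SimpleMovingObject is an environment actor that moves its static mesh back and forth along a spline.
; Each tick and on construction, it derives looping progress from server world time plus first-player ping, reversing on alternate cycles to keep clients in sync without moving the mesh incrementally.
; A float curve shapes that progress before constant-velocity spline sampling.
; The authority records MovementStartTime at BeginPlay, but the movement calculation never reads it.
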(event EventBeginPlay
  (Networking|SwitchHasAuthority
    (:Authority
      (Variables|State|SetMovementStartTime (GameState|GetServerWorldTimeSeconds (Game|GetGameState))))))

(event EventTick
  (params (DeltaSeconds :type Float%20%28single-precision%29))
  (CallFunction|RefreshMeshLocation))

(fn ConstructionScript
  (|CallParentFunction)
  (Variables|/Script/Engine.SplineComponent|SetDuration (Variables|Default|GetMovementSpline) (Variables|Settings|SimpleMovingObject|GetMovementDuration))
  (CallFunction|RefreshMeshLocation))

(fn RefreshMeshLocation
  (Utilities|IsValid (Game|GetGameState)
    (:Is%20Valid
      (LocalVariables|SetMovementTimeRatio (/ (+ (GameState|GetServerWorldTimeSeconds (Game|GetGameState)) (Class|AlsUtility|GetFirstPlayerPingSeconds)) (Variables|/Script/Engine.SplineComponent|GetDuration (Variables|Default|GetMovementSpline))))
      (LocalVariables|SetbInverseMovement (!= (Math|Integer|%(Integer) (Math|Float|Floor (LocalVariables|GetMovementTimeRatio)) 2) 0))
      (Transformation|SetWorldLocation (Variables|Default|GetStaticMesh) (Spline|GetLocationatTime (Variables|Default|GetMovementSpline) (* (Math|Curves|GetFloatValue (Variables|Settings|SimpleMovingObject|GetMovementCurve) (Math|Float|SelectFloat (- 1.0 (Math|Float|%(Float) (LocalVariables|GetMovementTimeRatio) 1.0)) (Math|Float|%(Float) (LocalVariables|GetMovementTimeRatio) 1.0) (LocalVariables|GetbInverseMovement))) (Variables|/Script/Engine.SplineComponent|GetDuration (Variables|Default|GetMovementSpline))) "World" true) false false))))