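; BP_SimpleObject is a configurable environment prop in the ALS extras that displays a chosen mesh and material.
; Its construction script assigns both from variables, with the material going to the first slot only.
; It then pushes top and side color pairs and a tiling value as material parameters, so each instance can be styled individually.
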(fn ConstructionScript
  (Components|StaticMesh|SetStaticMesh (Variables|Default|GetStaticMesh) (Variables|Settings|SimpleObject|GetMesh))
  (Rendering|Material|SetMaterial (Variables|Default|GetStaticMesh) 0 (Variables|Settings|SimpleObject|GetMaterial))
  (Rendering|Material|SetVectorParameterValueonMaterials (Variables|Default|GetStaticMesh) "TopColorA" (Math|Conversions|ToVector(LinearColor) (Variables|Settings|SimpleObject|GetTopColorA)))
  (Rendering|Material|SetVectorParameterValueonMaterials (Variables|Default|GetStaticMesh) "TopColorB" (Math|Conversions|ToVector(LinearColor) (Variables|Settings|SimpleObject|GetTopColorB)))
  (Rendering|Material|SetVectorParameterValueonMaterials (Variables|Default|GetStaticMesh) "SideColorA" (Math|Conversions|ToVector(LinearColor) (Variables|Settings|SimpleObject|GetSideColorA)))
  (Rendering|Material|SetVectorParameterValueonMaterials (Variables|Default|GetStaticMesh) "SideColorB" (Math|Conversions|ToVector(LinearColor) (Variables|Settings|SimpleObject|GetSideColorB)))
  (Rendering|Material|SetScalarParameterValueonMaterials (Variables|Default|GetStaticMesh) "Tiling" (Variables|Settings|SimpleObject|GetTiling)))