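; BP_SimpleRotatingObject is an environment actor that rotates continuously at a set RotationSpeed.
; Each Tick sets an absolute actor rotation from RotationSpeed multiplied by server world time plus the first player's ping in seconds, once the GameState is valid.
; Deriving rotation from the shared clock, rather than accumulating delta time, lets each machine compute it locally with latency compensation.
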(event EventTick
  (params (DeltaSeconds :type Float%20%28single-precision%29))
  (|CallParentFunction DeltaSeconds)
  (CallFunction|RefreshMeshRotation))

(fn ConstructionScript
  (|CallParentFunction))

(fn RefreshMeshRotation
  (Utilities|IsValid (Game|GetGameState)
    (:Is%20Valid
      (Transformation|SetActorRotation (* (Variables|Settings|SimpleRotatingObject|GetRotationSpeed) (+ (GameState|GetServerWorldTimeSeconds (Game|GetGameState)) (Class|AlsUtility|GetFirstPlayerPingSeconds)))))))