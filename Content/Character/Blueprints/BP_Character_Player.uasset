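; Player character Blueprint built on ALS, adding overlay-driven held items and GAS melee combat.
; Overlay mode changes relink animation layers and re-attach hand props, which also clear during ragdoll and non-low mantles; overlay also selects low-mantle settings.
; While CanHit is set, the locally controlled player box-traces between right-hand weapon sockets.
; Each newly hit actor triggers the melee ability and a damage gameplay event, with zero-distance hits flagged as reflected.
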(event Input|EnhancedActionEvents|EnhancedInputActionIA_Als_Interact
  (params (ActionValue :type Boolean) (ElapsedSeconds :type Float%20%28double-precision%29) (TriggeredSeconds :type Float%20%28double-precision%29) (InputAction :type Input%20Action%20Object%20Reference :default "/ALS/ALS/Data/Input/IA_Als_Interact.IA_Als_Interact"))
  ;[1 1 1] 测试用，F键触发
  (:Started
    (Variables|Default|SetbInteracting true)
    ;[1 1 1] 拿出武器动画，后面改到GAS
    (Animation|PlayAnimMontage "/ALS/ALS/Animations/Actions/Melee/AM_Als_Equip_Melee_Back.AM_Als_Equip_Melee_Back" 1.0 "None"))
  (:Completed
    (Variables|Default|SetbInteracting false)))

(event EventOnAttackStateChanged
  (params (PreviousAttackState :type Gameplay%20Tag%20Structure%20%28by%20ref%29)))

(event EventOnOverlayModeChanged
  (params (PreviousOverlayMode :type Gameplay%20Tag%20Structure%20%28by%20ref%29))
  (Overlay|RefreshOverlayLinkedAnimationLayer)
  (Overlay|ClearOverlayObject)
  (Overlay|SetupOverlayObject))

(event EventOnMantlingEnded
  (Overlay|SetupOverlayObject))

(event EventOnRagdollingEnded
  (Overlay|SetupOverlayObject))

(event EventOnMantlingStarted
  (params (Parameters :type Als%20Mantling%20Parameters%20Structure%20%28by%20ref%29))
  (if (Utilities|Enum|NotEqual(Enum) (.mantlingtype Parameters) "Low")
    (Overlay|ClearOverlayObject)))

(event EventBeginPlay
  (bind _abilitysystemcomponent (Variables|Default|GetAbilitySystemComponent))
  (Overlay|SetupOverlayObject)
  (GameplayAbilities|GiveAbility _abilitysystemcomponent "/ALS/Character/GAS/GA_MeleeAttack.GA_MeleeAttack_C" 0 -1)
  (GameplayAbilities|GiveAbility _abilitysystemcomponent "/ALS/Character/GAS/GA_Test.GA_Test_C" 0 -1))

(event EventOnRagdollingStarted
  (Overlay|ClearOverlayObject))

(event EventTick
  (params (DeltaSeconds :type Float%20%28single-precision%29))
  (if (Pawn|IsLocallyControlled)
    (if (Variables|Default|GetbCanHit)
      (bind _resultvalue (CallFunction|HitDetection (Variables|Default|GetOverlayStaticMesh_R)))
      (if _resultvalue
        (Utilities|FlowControl|Delay 0.2)
        (if (Variables|Default|GetbHitting)
          (Variables|Default|SetbHitting false)
          (Variables|Default|SetbHitReflected false))))))

(fn ConstructionScript
  (Components|SkinnedMesh|SetLeaderPoseComponent (Variables|Default|GetFullBody) (Variables|Character|GetMesh) false false))

(fn RefreshOverlayLinkedAnimationLayer
  (bind _mesh (Variables|Character|GetMesh))
  (LocalVariables|SetOverlayAnimationInstanceClass (.Value (Utilities|Map|Find (Variables|AlsCharacter|GetOverlayAnimationInstanceClasses) (Variables|Default|GetOverlayMode))))
  (bind _overlayanimationinstanceclass (LocalVariables|GetOverlayAnimationInstanceClass)
    (:then
      (Components|SkeletalMesh|AnimationBlueprintLinking|LinkAnimClassLayers _mesh _overlayanimationinstanceclass))
    (:else
      (Components|SkeletalMesh|AnimationBlueprintLinking|LinkAnimClassLayers _mesh "/ALS/ALS/Character/AnimationInstances/Overlays/AB_Als_Default.AB_Als_Default_C"))))

(fn RefreshOverlayObjecttoDelete
  (|SwitchGameplayTag (Variables|Default|GetOverlayMode)
    (:Default
      (Overlay|ClearOverlayObject))
    (:Als.OverlayMode.Rifle
      (Overlay|AttachOverlayObjecttoDelete 0 "/ALS/ALS/OverlayObjects/Rifle/SKM_Als_Rifle.SKM_Als_Rifle" 0 "Rifle" false))
    (:Als.OverlayMode.PistolOneHanded
      (Overlay|AttachOverlayObjecttoDelete 0 "/ALS/ALS/OverlayObjects/Pistol/SKM_Als_Pistol.SKM_Als_Pistol" 0 "Pistol_1h" false))
    (:Als.OverlayMode.PistolTwoHanded
      (Overlay|AttachOverlayObjecttoDelete 0 "/ALS/ALS/OverlayObjects/Pistol/SKM_Als_Pistol.SKM_Als_Pistol" 0 "Pistol" false))
    (:Als.OverlayMode.Bow
      (Overlay|AttachOverlayObjecttoDelete 0 "/ALS/ALS/OverlayObjects/Bow/SKM_Als_Bow.SKM_Als_Bow" "/ALS/ALS/OverlayObjects/Bow/AB_Als_Bow.AB_Als_Bow_C" "Bow" true))
    (:Als.OverlayMode.Torch
      (Overlay|AttachOverlayObjecttoDelete "/ALS/ALS/OverlayObjects/Torch/SM_Als_Torch.SM_Als_Torch" 0 0 "Torch" true))
    (:Als.OverlayMode.Binoculars
      (Overlay|AttachOverlayObjecttoDelete "/ALS/ALS/OverlayObjects/Binoculars/SM_Als_Binoculars.SM_Als_Binoculars" 0 0 "Binoculars" false))
    (:Als.OverlayMode.Box
      (Overlay|AttachOverlayObjecttoDelete "/ALS/ALS/OverlayObjects/Box/SM_Als_Box.SM_Als_Box" 0 0 "Box" false))
    (:Als.OverlayMode.Barrel
      (Overlay|AttachOverlayObjecttoDelete "/ALS/ALS/OverlayObjects/Barrel/SM_Als_Barrel.SM_Als_Barrel" 0 0 "Barrel" true))
    (:Als.OverlayMode.MeleeOneHanded
      (Overlay|AttachOverlayObjecttoDelete 0 0 0 "Melee_1h" false))))

(fn AttachOverlayObjecttoDelete
  (params (InputStaticMesh :type Static%20Mesh%20Object%20Reference) (InputSkeletalMesh :type Skeletal%20Mesh%20Object%20Reference) (InputAnimationClass :type Anim%20Instance%20Class%20Reference) (SocketName :type Name) (bUseLeftGunBone :type Boolean))
  (LocalVariables|SetResultSocketName (select (Variables|AlsCharacter|GetbUseGunBoneForOverlayObjects) (select bUseLeftGunBone (Class|AlsConstants|HandLeftGunVirtualBoneName) (Class|AlsConstants|HandRightGunVirtualBoneName)) SocketName))
  (Utilities|FlowControl|Sequence
    (:then_0
      (Components|StaticMesh|SetStaticMesh (Variables|Default|GetOverlayStaticMesh_L) InputStaticMesh)
      (Transformation|AttachComponentToComponent (Variables|Default|GetOverlayStaticMesh_L) (Variables|Character|GetMesh) (LocalVariables|GetResultSocketName) "SnapToTarget" "SnapToTarget" "SnapToTarget" true))
    (:then_1
      (Components|SkinnedMesh|SetSkinnedAssetandUpdate (Variables|Default|GetOverlaySkeletalMesh_L) InputSkeletalMesh true)
      (Class|SkeletalMeshComponent|SetAnimClass (Variables|Default|GetOverlaySkeletalMesh_L) InputAnimationClass)
      (Transformation|AttachComponentToComponent (Variables|Default|GetOverlaySkeletalMesh_L) (Variables|Character|GetMesh) (LocalVariables|GetResultSocketName) "SnapToTarget" "SnapToTarget" "SnapToTarget" true))))

(fn ClearOverlayObject
  (Utilities|FlowControl|Sequence
    (:then_0
      (Components|StaticMesh|SetStaticMesh (Variables|Default|GetOverlayStaticMesh_L) 0)
      (Components|SkinnedMesh|SetSkinnedAssetandUpdate (Variables|Default|GetOverlaySkeletalMesh_L) 0 true)
      (Class|SkeletalMeshComponent|SetAnimClass (Variables|Default|GetOverlaySkeletalMesh_L)))
    (:then_1
      (Components|StaticMesh|SetStaticMesh (Variables|Default|GetOverlayStaticMesh_R) 0)
      (Components|SkinnedMesh|SetSkinnedAssetandUpdate (Variables|Default|GetOverlaySkeletalMesh_R) 0 true)
      (Class|SkeletalMeshComponent|SetAnimClass (Variables|Default|GetOverlaySkeletalMesh_R)))))

(fn SelectMantlingSettings
  (params (MantlingType :type EAlsMantlingType%20Enum :default "High"))
  (switch Utilities|FlowControl|Switch|SwitchonEAlsMantlingType MantlingType
    (:High
      _)
    (:Low
      (|SwitchGameplayTag (Variables|Default|GetOverlayMode)
        (:Default
          (return "/ALS/ALS/Data/Character/Mantle/MS_Als_Low.MS_Als_Low"))
        (:Als.OverlayMode.Injured
          _)
        (:Als.OverlayMode.HandsTied
          (return "/ALS/ALS/Data/Character/Mantle/MS_Als_Low_BothHands.MS_Als_Low_BothHands"))
        (:Als.OverlayMode.Rifle
          (return "/ALS/ALS/Data/Character/Mantle/MS_Als_Low_Right.MS_Als_Low_Right"))
        (:Als.OverlayMode.PistolOneHanded
          (return "/ALS/ALS/Data/Character/Mantle/MS_Als_Low_Right.MS_Als_Low_Right"))
        (:Als.OverlayMode.PistolTwoHanded
          (return "/ALS/ALS/Data/Character/Mantle/MS_Als_Low_Right.MS_Als_Low_Right"))
        (:Als.OverlayMode.Bow
          _)
        (:Als.OverlayMode.Torch
          _)
        (:Als.OverlayMode.Binoculars
          (return "/ALS/ALS/Data/Character/Mantle/MS_Als_Low_Right.MS_Als_Low_Right"))
        (:Als.OverlayMode.Box
          (return "/ALS/ALS/Data/Character/Mantle/MS_Als_Low_Box.MS_Als_Low_Box"))
        (:Als.OverlayMode.Barrel
          _))
      (return "/ALS/ALS/Data/Character/Mantle/MS_Als_Low_Left.MS_Als_Low_Left"))
    (:InAir
      _))
  (return "/ALS/ALS/Data/Character/Mantle/MS_Als_High.MS_Als_High"))

(fn SetupOverlayObject
  (|SwitchGameplayTag (Variables|Default|GetOverlayMode)
    (:Default
      (Overlay|ClearOverlayObject))
    (:Als.OverlayMode.Rifle
      (Overlay|AssignOverlayObject 0 "/ALS/ALS/OverlayObjects/Rifle/SKM_Als_Rifle.SKM_Als_Rifle" 0 "Rifle" (Variables|Default|GetOverlayStaticMesh_R) (Variables|Default|GetOverlaySkeletalMesh_R) false))
    (:Als.OverlayMode.PistolOneHanded
      (Overlay|AssignOverlayObject 0 "/ALS/ALS/OverlayObjects/Pistol/SKM_Als_Pistol.SKM_Als_Pistol" 0 "Pistol_1h" (Variables|Default|GetOverlayStaticMesh_R) (Variables|Default|GetOverlaySkeletalMesh_R) false))
    (:Als.OverlayMode.Bow
      (Overlay|AssignOverlayObject 0 "/ALS/ALS/OverlayObjects/Bow/SKM_Als_Bow.SKM_Als_Bow" "/ALS/ALS/OverlayObjects/Bow/AB_Als_Bow.AB_Als_Bow_C" "Bow" (Variables|Default|GetOverlayStaticMesh_L) (Variables|Default|GetOverlaySkeletalMesh_L) true))
    (:Als.OverlayMode.MeleeOneHanded
      (Overlay|AssignOverlayObject "/Game/Packs/Weapon_Pack/Mesh/Weapons/Weapons_Kit/SM_Sword.SM_Sword" 0 0 "Melee_1h" (Variables|Default|GetOverlayStaticMesh_R) (Variables|Default|GetOverlaySkeletalMesh_R) false))
    (:Als.OverlayMode.Default
      (Overlay|AssignOverlayObject 0 0 0 "None" (Variables|Default|GetOverlayStaticMesh_R) (Variables|Default|GetOverlaySkeletalMesh_R) false))))

(fn AssignOverlayObject
  (params (InputStaticMesh :type Static%20Mesh%20Object%20Reference) (InputSkeletalMesh :type Skeletal%20Mesh%20Object%20Reference) (InputAnimInstance :type Anim%20Instance%20Class%20Reference) (InputSocketName :type Name) (InputOverlayStaticMesh :type Static%20Mesh%20Component%20Object%20Reference) (InputOverlaySkeletalMesh :type Skeletal%20Mesh%20Component%20Object%20Reference) (UseLeftGunBone :type Boolean))
  (LocalVariables|SetResultSocketName (select (Variables|AlsCharacter|GetbUseGunBoneForOverlayObjects) (select UseLeftGunBone (Class|AlsConstants|HandLeftGunVirtualBoneName) (Class|AlsConstants|HandRightGunVirtualBoneName)) InputSocketName))
  (Utilities|FlowControl|Sequence
    (:then_0
      (Components|StaticMesh|SetStaticMesh InputOverlayStaticMesh InputStaticMesh)
      (Transformation|AttachComponentToComponent InputOverlayStaticMesh (Variables|Character|GetMesh) (LocalVariables|GetResultSocketName) "SnapToTarget" "SnapToTarget" "SnapToTarget" true))
    (:then_1
      (Components|SkinnedMesh|SetSkinnedAssetandUpdate InputOverlaySkeletalMesh InputSkeletalMesh true)
      (Class|SkeletalMeshComponent|SetAnimClass InputOverlaySkeletalMesh InputAnimInstance) ; 应用武器动画蓝图
      (Transformation|AttachComponentToComponent InputOverlaySkeletalMesh (Variables|Character|GetMesh) (LocalVariables|GetResultSocketName) "SnapToTarget" "SnapToTarget" "SnapToTarget" true))))

(fn HitDetection
  (params (InputComponent :type Mesh%20Component%20Object%20Reference))
  (bind _returnvalue (Class|AlsCharacter|CalculateSweepTraceParameters InputComponent "Start" "End"))
  (bind _self self)
  (bind _outhit (Class|KismetSystemLibrary|BoxTraceSingleforObjects (.start _returnvalue) (.end _returnvalue) (.halfsize _returnvalue) (.rotator _returnvalue) (Utilities|Array|MakeArray "ObjectTypeQuery1" "ObjectTypeQuery2" "ObjectTypeQuery4" "ObjectTypeQuery5") false 0 "None" true "(R=1.000000,G=0.000000,B=0.000000,A=1.000000)" "(R=0.000000,G=1.000000,B=0.000000,A=1.000000)" 1.0))
  (bind _output_get (LocalVariables|SetOutHitBlocked (.bblockinghit _outhit)))
  (if _output_get
    (if (not (Utilities|Array|ContainsItem (Variables|Default|GetHittingActor) (.hitactor _outhit)))
      (Variables|Default|SetbHitReflected (== (.distance _outhit) 0.0))
      (Utilities|Array|Add (Variables|Default|GetHittingActor) (.hitactor _outhit))
      (Variables|Default|SetbHitting true)
      (Abilities|TryActivateAbilitybyClass (Variables|Default|GetAbilitySystemComponent) "/ALS/Character/GAS/GA_MeleeAttack.GA_MeleeAttack_C" true)
      (Ability|SendGameplayEventtoActor _self "(TagName=\"Event.Damage\")" (Utilities|Struct|MakeGameplayEventData "(TagName=\"Event.Damage\")" _self (.hitactor _outhit)))
      (Development|PrintString (Utilities|String|ToString(Boolean) (Variables|Default|GetbCanHit)) false false)
      (Development|PrintString (Utilities|String|ToString(Boolean) (Variables|Default|GetbHitting)) false false "(R=0.000000,G=1.000000,B=0.521003,A=1.000000)")
      (Development|PrintString (Utilities|String|ToString(Boolean) (Variables|Default|GetbHitReflected)) false false "(R=1.000000,G=0.043060,B=0.000000,A=1.000000)")
      (return true)
      (else
        _)))
  (return false))