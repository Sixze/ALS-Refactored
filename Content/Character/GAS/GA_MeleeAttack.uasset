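; GA_MeleeAttack is a Gameplay Ability that deals melee damage when signalled by a gameplay event.
; On activation it commits, then waits for Event.Damage, or ends at once if the commit fails.
; The event payload supplies Instigator and Target, whose ability system components apply GE_DealDamage before the ability ends with a debug print.
; Montage playback and backward root-motion force nodes are present but unconnected, so neither runs.
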(event Ability|EventActivateAbility
  (bind _returnvalue (Ability|CommitAbility))
  (if _returnvalue
    (bind _payload (Ability|Tasks|WaitGameplayEvent "(TagName=\"Event.Damage\")" 0)
      (:EventReceived
        (GameplayEffects|ApplyGameplayEffectToTarget :self (Ability|GetAbilitySystemComponent (.Instigator (Utilities|Struct|BreakGameplayEventData _payload))) :GameplayEffectClass "/ALS/Character/GAS/GE_DealDamage.GE_DealDamage_C" :Target (Ability|GetAbilitySystemComponent (.Target (Utilities|Struct|BreakGameplayEventData _payload))))
        (Ability|EndAbility)))
    (else
      (Ability|EndAbility))))

(event Ability|EventOnEndAbility
  (params (bWasCancelled :type Boolean))
  (Development|PrintString "End" true false))