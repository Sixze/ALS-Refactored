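; GA_Test is a test gameplay ability that shoves its avatar backward in a short dash.
; On activation it commits, then runs an ApplyRootMotionConstantForce task along the negated forward vector, keeping the last root motion velocity when it finishes.
; The ability ends when the task finishes or immediately if the commit fails, and prints a debug message on end.
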(event Ability|EventActivateAbility
  (bind _returnvalue (Ability|CommitAbility))
  (if _returnvalue
    (Ability|Tasks|ApplyRootMotionConstantForce "None" (* (Transformation|GetActorForwardVector (Ability|GetAvatarActorfromActorInfo)) -1.0) 3e+02 0.1 false 0 "MaintainLastRootMotionVelocity"
      (:OnFinish
        (Ability|EndAbility)))
    (else
      (Ability|EndAbility))))

(event Ability|EventOnEndAbility
  (params (bWasCancelled :type Boolean))
  (Development|PrintString "End" true false))